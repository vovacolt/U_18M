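; Blueprint function library for the resource-based building system, handling affordability checks and Russian-language build tooltips.
; A shared parser flattens a resource struct into a map keyed by resource type.
; The requirement check tests negative Need entries against the player pawn's ResStorage.
; The tooltip builder lists nonzero, localized, signed amounts for construction (Need) and per-turn yield (Give) in a UI_Base_Sq_ToolTip widget.
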(fn `Build_ST_Parser`
  (params (Structure :type "/Game/Blueprints/ST_Requirements Structure"))
  (returns (Resurses :type "Map of /Game/Blueprints/E_Requirements Enum to Integer"))
  (locals (Local_Res :type "Map of /Game/Blueprints/E_Requirements Enum to Integer"))
  (bind (_organic _non_organic _stimulants _bodies _humans _mechanics _energy) (break `/Game/Blueprints/ST_Requirements` Structure))
  (bind _local_res (`local.Local_Res`))
  (`|ExecutionSequence`
    (:`then_0`
      (`BlueprintMapLibrary.Map_Add` _local_res "NewEnumerator0" _organic))
    (:`then_1`
      (`BlueprintMapLibrary.Map_Add` _local_res "NewEnumerator1" _non_organic))
    (:`then_2`
      (`BlueprintMapLibrary.Map_Add` _local_res "NewEnumerator2" _stimulants))
    (:`then_3`
      (`BlueprintMapLibrary.Map_Add` _local_res "NewEnumerator3" _bodies))
    (:`then_4`
      (`BlueprintMapLibrary.Map_Add` _local_res "NewEnumerator4" _humans))
    (:`then_5`
      (`BlueprintMapLibrary.Map_Add` _local_res "NewEnumerator5" _mechanics))
    (:`then_6`
      (`BlueprintMapLibrary.Map_Add` _local_res "NewEnumerator6" _energy))
    (:`then_7`
      (return _local_res))))

(fn `Check_Build_Requiments`
  (params (ST_Buildings :type "/Game/Blueprints/ST_Buildings Structure (by ref)"))
  (returns (Out :type Boolean))
  (bind _resurses (`self.Build_ST_Parser` (`.Need_6_FC49DD6D40EB4853A6AA3CAF8A0AB544` (break `/Game/Blueprints/ST_Buildings` ST_Buildings))))
  (bind _asbp_default_pawn (cast `/Game/Blueprints/BP_Default_Pawn` (`GameplayStatics.GetPlayerPawn` null)))
  (bind _res_storage (`/Game/Blueprints/BP_Default_Pawn.Res_Storage` _asbp_default_pawn))
  (bind _keys (`BlueprintMapLibrary.Map_Keys` _res_storage))
  (for _array_element _keys
    (bind _value (`BlueprintMapLibrary.Map_Find` _resurses _array_element))
    (if (and (< _value 0) (< (+ _value (`BlueprintMapLibrary.Map_Find` _res_storage _array_element)) 0))
      (return false)))
  (return true))

(fn `Filling_In_ToolTip`
  (params (ST_Buildings :type "/Game/Blueprints/ST_Buildings Structure (by ref)") (InString :type String))
  (returns (Out_Widget :type "/Game/UI_UX/ToolTips/UI_Base_Sq_ToolTip Object Reference"))
  (locals (Base_String_1 :type String) (Base_String_2 :type String))
  (bind (_class_ref _need _give) (break `/Game/Blueprints/ST_Buildings` ST_Buildings))
  (`|ExecutionSequence`
    (:`then_0`
      (bind _out (`self.ParseST_ToolTip` _need))
      (set `local.Base_string_1` _out))
    (:`then_1`
      (bind _out_2 (`self.ParseST_ToolTip` _give))
      (set `local.Base_string_2` _out_2))
    (:`then_2`
      (bind _returnvalue (`|CreateWidget` "/Game/UI_UX/ToolTips/UI_Base_Sq_ToolTip.UI_Base_Sq_ToolTip_C"))
      (`|ExecutionSequence`
        (:`then_0`
          (`TextBlock.SetText` (`/Game/UI_UX/ToolTips/UI_Base_Sq_ToolTip.ToolTip_Text_Name` _returnvalue) (`KismetTextLibrary.Conv_StringToText` InString)))
        (:`then_1`
          (`TextBlock.SetText` (`/Game/UI_UX/ToolTips/UI_Base_Sq_ToolTip.ToolTip_Text_1` _returnvalue) "Строительство:"))
        (:`then_2`
          (`TextBlock.SetText` (`/Game/UI_UX/ToolTips/UI_Base_Sq_ToolTip.ToolTip_Text_Info_1` _returnvalue) (`KismetTextLibrary.Conv_StringToText` (`KismetStringLibrary.TrimTrailing` (`local.Base_string_1`)))))
        (:`then_3`
          (`TextBlock.SetText` (`/Game/UI_UX/ToolTips/UI_Base_Sq_ToolTip.ToolTip_Text_2` _returnvalue) " \nВ ход:"))
        (:`then_4`
          (`TextBlock.SetText` (`/Game/UI_UX/ToolTips/UI_Base_Sq_ToolTip.ToolTip_Text_Info_2` _returnvalue) (`KismetTextLibrary.Conv_StringToText` (`KismetStringLibrary.TrimTrailing` (`local.Base_string_2`)))))
        (:`then_5`
          (return _returnvalue))))))

(fn `Localization_E_Requirements`
  (params (In :type "/Game/Blueprints/E_Requirements Enum" :default "NewEnumerator0"))
  (returns (Localization :type Name))
  (switch `/Game/Blueprints/E_Requirements` In
    (:`NewEnumerator0`
      (return "Органика"))
    (:`NewEnumerator1`
      (return "Неорганика"))
    (:`NewEnumerator2`
      (return "Стимуляторы"))
    (:`NewEnumerator3`
      (return "Оболочки"))
    (:`NewEnumerator4`
      (return "Люди"))
    (:`NewEnumerator5`
      (return "Киборги"))
    (:`NewEnumerator6`
      (return "Энергия"))))

(fn `ParseST_ToolTip`
  (params (Structure :type "/Game/Blueprints/ST_Requirements Structure"))
  (returns (Out :type String))
  (locals (Out_Local :type String))
  (bind _resurses (`self.Build_ST_Parser` Structure))
  (bind _keys (`BlueprintMapLibrary.Map_Keys` _resurses))
  (for _array_element _keys
    (bind _value (`BlueprintMapLibrary.Map_Find` _resurses _array_element))
    (if (!= _value 0)
      (bind _localization (`self.Localization_E_Requirements` _array_element))
      (set `local.Out_Local` (`KismetStringLibrary.Concat_StrStr` (`local.Out_Local`) (`KismetStringLibrary.Conv_NameToString` _localization) ": " (`KismetTextLibrary.Conv_TextToString` (select `bool` (> _value 0) :`false` (`KismetTextLibrary.Conv_IntToText` _value) :`true` (`|FormatText` "+{0}" _value))) " \n"))))
  (return (`local.Out_Local`)))
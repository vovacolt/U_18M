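; Default player pawn for a day-based resource builder, handling camera orbit and zoom, building placement and the HUD.
; Placing a building via CBuildComponent applies its cost and yield to storage and growth maps, then advances the day.
; Skipping a day, allowed after early days, incurs a doubling resource penalty.
; Each turn applies growth, checks two loss conditions, then shows that day's DT_Dialogs entry and checks for victory.
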(event `self.ReceiveBeginPlay`
  (`|ExecutionSequence`
    (:`then_0`
      (bind _returnvalue (`|CreateWidget` "/Game/UI_UX/HUB/UI_Game_Hub.UI_Game_Hub_C"))
      (`UserWidget.AddToViewport` _returnvalue 0)
      (`WidgetBlueprintLibrary.SetInputMode_GameAndUIEx` (`GameplayStatics.GetPlayerController` 0) _returnvalue "LockAlways" false)
      (`self.Spawn_Dialogs`))
    (:`then_1`
      (`KismetSystemLibrary.Delay` 1.0)
      (bind _astop_down_controller (cast `/Game/TopDownBP/Blueprints/TopDownController` (`GameplayStatics.GetPlayerController` 0)))
      (set `/Game/TopDownBP/Blueprints/TopDownController.Load_Level` true _astop_down_controller))))

(event `self.ReceiveTick`
  (params (DeltaSeconds :type "Float (single-precision)"))
  (bind _camera (`self.Camera`))
  (bind (_returnvalue_roll _returnvalue_pitch _returnvalue_yaw) (`KismetMathLibrary.BreakRotator` (`SceneComponent.K2_GetComponentRotation` _camera)))
  (bind (_returnvalue_roll_2 _returnvalue_pitch_2 _returnvalue_yaw_2) (`KismetMathLibrary.BreakRotator` (`SceneComponent.K2_GetComponentRotation` _camera)))
  (`|ExecutionSequence`
    (:`then_0`
      (`/Engine/EditorBlueprintResources/StandardMacros.Gate` true :!label _label
        (:`Exit`
          (`SceneComponent.K2_SetWorldRotation` (`self.SpringArm`) (`KismetMathLibrary.MakeRotator` _returnvalue_roll _returnvalue_pitch (+ _returnvalue_yaw (`self.Camera_Rot_Angle`))) false false))))
    (:`then_1`
      (`/Engine/EditorBlueprintResources/StandardMacros.Gate` true :!label _label_2
        (:`Exit`
          (`SceneComponent.K2_SetWorldRotation` (`self.SpringArm`) (`KismetMathLibrary.MakeRotator` _returnvalue_roll_2 _returnvalue_pitch_2 (- _returnvalue_yaw_2 (`self.Camera_Rot_Angle`))) false false))))))

(event `Key|Q`
  (params (Key :type "Key Structure"))
  (:`Pressed`
    (goto _label :!via `Open`))
  (:`Released`
    (goto _label :!via `Close`)))

(event `InputAction|Interaction`
  (params (Key :type "Key Structure"))
  (bind (_class_ref _need _give) (break `/Game/Blueprints/ST_Buildings` (`self.Building`)))
  (:`Pressed`
    (if (and (not (`/Game/Blueprints/Components/Build_Component/C_Build_Component.Blocking_Hit` (`self.C_Build_Component`))) (`self.Now_Placing`))
      (`/Game/Blueprints/Components/Build_Component/C_Build_Component.Finish_Set_Construction` (`self.C_Build_Component`))
      (`self.On Build Action` _need _give)
      (`self.Build_Action_Grow`)
      (`/Engine/EditorBlueprintResources/StandardMacros.IncrementInt` (`self.Current_Day`)
        (:`  `
          (set `self.Now_Placing` false)
          (set `self.Building` (struct))
          (bind _out (`self.On_Death_GameOver`))
          (if _out
            (bind _returnvalue (`|CreateWidget` "/Game/UI_UX/UI_GameOver_1.UI_GameOver_1_C"))
            (`UserWidget.AddToViewport` _returnvalue 0)
            (else
              (`self.On_ResOver_GameOver`)
              (if (> (`self.Death_Score`) (`self.Max_Death_Score`))
                (bind _returnvalue_2 (`|CreateWidget` "/Game/UI_UX/UI_GameOver_2.UI_GameOver_2_C"))
                (`UserWidget.AddToViewport` _returnvalue_2 0)
                (else
                  (`self.Spawn_Dialogs`)
                  (`self.Win`))))))))))

(event `Key|E`
  (params (Key :type "Key Structure"))
  (:`Pressed`
    (goto _label_2 :!via `Open`))
  (:`Released`
    (goto _label_2 :!via `Close`)))

(event `Key|MouseScrollDown`
  (params (Key :type "Key Structure"))
  (bind _springarm (`self.SpringArm`))
  (bind _returnvalue (+ (`SpringArmComponent.TargetArmLength` _springarm) (`self.Scope`)))
  (:`Pressed`
    (if (`self.Now_Placing`)
      (`/Game/Blueprints/Components/Build_Component/C_Build_Component.Rotate_Construction` (`self.C_Build_Component`) true)
      (elif (< _returnvalue (`self.Max_Scope`))
        (set `SpringArmComponent.TargetArmLength` _returnvalue _springarm)))))

(event `Key|RightMouseButton`
  (params (Key :type "Key Structure"))
  (:`Pressed`
    (if (`self.Now_Placing`)
      (`/Game/Blueprints/Components/Build_Component/C_Build_Component.Cancel_Building` (`self.C_Build_Component`))
      (elif (> (`self.Current_Day`) 3)
        (`/Engine/EditorBlueprintResources/StandardMacros.IncrementInt` (`self.Current_Day`)
          (:`  `
            (set `self.Skip_Score` (* (`self.Skip_Score`) 2))
            (`self.Panishment`)
            (`self.Build_Action_Grow`)
            (bind _out (`self.On_Death_GameOver`))
            (if _out
              (bind _returnvalue (`|CreateWidget` "/Game/UI_UX/UI_GameOver_1.UI_GameOver_1_C"))
              (`UserWidget.AddToViewport` _returnvalue 0)
              (else
                (`self.On_ResOver_GameOver`)
                (if (> (`self.Death_Score`) (`self.Max_Death_Score`))
                  (bind _returnvalue_2 (`|CreateWidget` "/Game/UI_UX/UI_GameOver_2.UI_GameOver_2_C"))
                  (`UserWidget.AddToViewport` _returnvalue_2 0)
                  (else
                    (`self.Spawn_Dialogs`)
                    (`self.Win`)))))))))))

(event `Key|MouseScrollUp`
  (params (Key :type "Key Structure"))
  (bind _springarm (`self.SpringArm`))
  (bind _returnvalue (- (`SpringArmComponent.TargetArmLength` _springarm) (`self.Scope`)))
  (:`Pressed`
    (if (`self.Now_Placing`)
      (`/Game/Blueprints/Components/Build_Component/C_Build_Component.Rotate_Construction` (`self.C_Build_Component`) false)
      (elif (> _returnvalue (`self.Min_Scope`))
        (set `SpringArmComponent.TargetArmLength` _returnvalue _springarm)))))

(fn `Build_Action_Grow`
  (locals (NewLocalVar_0 :type "/Game/Blueprints/ST_Requirements Structure"))
  (bind _res_storage (`self.Res_Storage`))
  (bind _keys (`BlueprintMapLibrary.Map_Keys` _res_storage))
  (for _array_element _keys
    (`BlueprintMapLibrary.Map_Add` _res_storage _array_element (+ (`BlueprintMapLibrary.Map_Find` _res_storage _array_element) (`BlueprintMapLibrary.Map_Find` (`self.Res_Grows`) _array_element)))))

(fn `Build_Action_Storage`
  (params (Struct :type "/Game/Blueprints/ST_Requirements Structure") (TargetMap :type "Map of /Game/Blueprints/E_Requirements Enum to Integer (by ref)"))
  (locals (NewLocalVar_0 :type "/Game/Blueprints/ST_Requirements Structure"))
  (bind _resurses (`/Game/Blueprints/BFL_Default.Build_ST_Parser` Struct))
  (bind _keys (`BlueprintMapLibrary.Map_Keys` TargetMap))
  (for _array_element _keys
    (`BlueprintMapLibrary.Map_Add` TargetMap _array_element (+ (`BlueprintMapLibrary.Map_Find` TargetMap _array_element) (`BlueprintMapLibrary.Map_Find` _resurses _array_element)))))

(fn `Get_Interaction_Info`
  (returns (Hit_Info :type "HitResult Structure"))
  (return (`PlayerController.GetHitResultUnderCursorByChannel` (`GameplayStatics.GetPlayerController` 0) "TraceTypeQuery1" true)))

(fn `On Build Action`
  (params (Need :type "/Game/Blueprints/ST_Requirements Structure") (Give :type "/Game/Blueprints/ST_Requirements Structure"))
  (`|ExecutionSequence`
    (:`then_0`
      (`self.Build_Action_Storage` Need (`self.Res_Storage`)))
    (:`then_1`
      (`self.Build_Action_Storage` Give (`self.Res_Grows`)))))

(fn `On_Death_GameOver`
  (returns (Out :type Boolean))
  (bind _res_storage (`self.Res_Storage`))
  (bind _res_grows (`self.Res_Grows`))
  (return (or (and (< (`BlueprintMapLibrary.Map_Find` _res_storage "NewEnumerator4") 0) (< (`BlueprintMapLibrary.Map_Find` _res_grows "NewEnumerator4") 0)) (and (< (`BlueprintMapLibrary.Map_Find` _res_storage "NewEnumerator5") 0) (< (`BlueprintMapLibrary.Map_Find` _res_grows "NewEnumerator5") 0)))))

(fn `On_ResOver_GameOver`
  (bind _res_storage (`self.Res_Storage`))
  (if (or (< (`BlueprintMapLibrary.Map_Find` _res_storage "NewEnumerator0") 0) (< (`BlueprintMapLibrary.Map_Find` _res_storage "NewEnumerator1") 0) (< (`BlueprintMapLibrary.Map_Find` _res_storage "NewEnumerator2") 0) (< (`BlueprintMapLibrary.Map_Find` _res_storage "NewEnumerator3") 0) (< (`BlueprintMapLibrary.Map_Find` _res_storage "NewEnumerator4") 0) (< (`BlueprintMapLibrary.Map_Find` _res_storage "NewEnumerator5") 0) (< (`BlueprintMapLibrary.Map_Find` _res_storage "NewEnumerator0") 0))
    (`/Engine/EditorBlueprintResources/StandardMacros.IncrementInt` (`self.Death_Score`))
    (else
      (set `self.Death_Score` 0))))

(fn `Panishment`
  (bind _res_storage (`self.Res_Storage`))
  (bind _skip_score (`self.Skip_Score`))
  (`BlueprintMapLibrary.Map_Add` _res_storage "NewEnumerator0" (- (`BlueprintMapLibrary.Map_Find` _res_storage "NewEnumerator0") _skip_score))
  (`BlueprintMapLibrary.Map_Add` _res_storage "NewEnumerator1" (- (`BlueprintMapLibrary.Map_Find` _res_storage "NewEnumerator1") _skip_score))
  (`BlueprintMapLibrary.Map_Add` _res_storage "NewEnumerator6" (- (`BlueprintMapLibrary.Map_Find` _res_storage "NewEnumerator6") _skip_score)))

(fn `Spawn_Dialogs`
  (bind _returnvalue (`|GetDataTableRow` "/Game/Blueprints/DT_Dialogs.DT_Dialogs" (`KismetStringLibrary.Conv_StringToName` (`KismetStringLibrary.Conv_IntToString` (`self.Current_Day`))))
    (:`then`
      (bind (_dialog_day _icon) (break `/Game/Blueprints/ST_Dialogs` _returnvalue))
      (bind _returnvalue_2 (`|CreateWidget` "/Game/UI_UX/Dialogs_and_Tasks/UI_DIalog.UI_DIalog_C" null _dialog_day _icon null))
      (`UserWidget.AddToViewport` _returnvalue_2 0))))

(fn `UserConstructionScript`)

(fn `Win`
  (if (== (`self.Current_Day`) (`self.Max_Days`))
    (bind _returnvalue (`|CreateWidget` "/Game/UI_UX/UI_Win_Main.UI_Win_Main_C"))
    (`UserWidget.AddToViewport` _returnvalue 0)))